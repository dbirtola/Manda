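; Player controller for Manda that creates the HUD on begin play and relays player input to the controlled BP_MandaPlayerNew pawn.
; Move, turn and Up/Down debug inputs pass through as messages, while SetControlMode switches between UI-only and game-only input with the cursor hidden in both.
; It also carries test code: sample debug-menu widgets that print changes, a debug menu toggle, a grab-bag randomizer on SpaceBar and a move-to-origin test input.
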(event Custom|Set%20Control%20Mode
  (params (Mouse%20Control :type Boolean) (FocusWidget :type User%20Widget%20Object%20Reference%20%28by%20ref%29))
  ;[1 1 1] Set control mode. Shows/hides mouse cursor and changes input mode accordingly
  (if Mouse%20Control
    (Input|SetInputModeUIOnly self FocusWidget "DoNotLock")
    (Variables|Default|SetbShowMouseCursor false)
    (else
      (Class|WidgetBlueprintLibrary|SetFocustoGameViewport)
      (Input|SetInputModeGameOnly self)
      (Variables|Default|SetbShowMouseCursor false))))

(event EventBeginPlay
  ;[1 1 1] Begin Play
  (bind _returnvalue (UserInterface|CreateWidget "/Game/Manda/UI/Widgets/HUD/WB_MandaHUD.WB_MandaHUD_C" self))
  (UserInterface|Viewport|AddtoViewport _returnvalue 0)
  (Variables|Default|SetManda%20HUD _returnvalue)
  (CallFunction|DEBUGDebugMenuTest)
  (CallFunction|Temp))

(event Custom|Temp
  (bind _output (Utilities|GrabBagRandomizer (Variables|Default|GetTempArray))
    (:ElementOut
      (Development|PrintString _output))))

(event Input|ActionEvents|InputActionOpenDebug
  (params (Key :type Key%20Structure))
  ;[1 1 1] Toggle Debug
  (:Pressed
    (bind _manda_hud (CallFunction|GetMandaHUD))
    (Utilities|IsValid _manda_hud
      (:Is%20Valid
        (Default|ToggleDebugMenu _manda_hud)))))

(event Input|AxisEvents|InputAxisMoveForward
  (params (AxisValue :type Float%20%28single-precision%29))
  ;[1 1 1] Toggle Debug
  (Class|BPMandaInputInterface|MoveForward(Message) (CallFunction|MandaPlayer) AxisValue))

(event Input|AxisEvents|InputAxisMoveRight
  (params (AxisValue :type Float%20%28single-precision%29))
  ;[1 1 1] Toggle Debug
  (Class|BPMandaInputInterface|MoveRight(Message) (CallFunction|MandaPlayer) AxisValue))

(event Input|AxisEvents|InputAxisTurnRight
  (params (AxisValue :type Float%20%28single-precision%29))
  ;[1 1 1] Toggle Debug
  (Class|BPMandaInputInterface|TurnRight(Message) (CallFunction|MandaPlayer) AxisValue))

(event Input|AxisEvents|InputAxisTurnUp
  (params (AxisValue :type Float%20%28single-precision%29))
  ;[1 1 1] Toggle Debug
  (Class|BPMandaInputInterface|TurnUp(Message) (CallFunction|MandaPlayer) AxisValue))

(event Input|KeyboardEvents|Up
  (params (Key :type Key%20Structure))
  ;[1 1 1] Toggle Debug
  (:Pressed
    (Class|BPMandaInputInterface|DebugIncrease(Message) (CallFunction|MandaPlayer))))

(event Input|KeyboardEvents|Down
  (params (Key :type Key%20Structure))
  ;[1 1 1] Toggle Debug
  (:Pressed
    (Class|BPMandaInputInterface|DebugDecrease(Message) (CallFunction|MandaPlayer))))

(event Input|KeyboardEvents|SpaceBar
  (params (Key :type Key%20Structure))
  (:Pressed
    (Utilities|GrabBagRandomizer (Variables|Default|GetTempArray)) ; enters at GetElement
  ))

(event Custom|DEBUG_OnEditableTextSubmited
  (params (Text :type Text%20%28by%20ref%29) (CommitMethod :type ETextCommit%20Enum :default "Default"))
  ;[1 0 0] [DEBUG] Testing debug stuff actually. Kindof interesting. If the debug stuff doesn't work, how do you debug that? Fuck.
  (Development|PrintText Text))

(event Custom|DEBUG_DebugMenuTest
  ;[1 0 0] [DEBUG] Testing debug stuff actually. Kindof interesting. If the debug stuff doesn't work, how do you debug that? Fuck.
  (Utilities|FlowControl|Sequence
    (:then_0
      (CallFunction|AddTextDebug "GAme Name" "Manda"))
    (:then_1
      (bind _editable_text_debug_widget (CallFunction|AddEditableTextDebug "Favorite Chip?" "Barbecue"))
      (EventDispatchers|BindEventtoOnTextCommitted (Variables|/Game/Manda/UI/Widgets/Debug/DebugMenuItems/WB_DebugEditableText.WB_DebugEditableText_C|GetValue _editable_text_debug_widget) (delegate Custom|DEBUG_OnEditableTextSubmited)))
    (:then_2
      (bind _combo_box_debug_widget (CallFunction|AddComboBoxDebug "Favorite Team Member" (Utilities|Array|MakeArray "Damen" "D. Birtola" "Mr. Birtola" "D-Man") "Damen"))
      (EventDispatchers|BindEventtoOnSelectionChanged (Variables|/Game/Manda/UI/Widgets/Debug/DebugMenuItems/WB_DebugComboBox.WB_DebugComboBox_C|GetValue _combo_box_debug_widget) (delegate Custom|DEBUG_OnComboSelectionChanged)))
    (:then_3
      (bind _checkbox_debug_widget (CallFunction|AddCheckboxDebug "Did you read the EULA?" true))
      (EventDispatchers|BindEventtoOnCheckStateChanged (Variables|/Game/Manda/UI/Widgets/Debug/DebugMenuItems/WB_DebugCheckbox.WB_DebugCheckbox_C|GetValue _checkbox_debug_widget) (delegate Custom|DEBUG_OnCheckboxStateChanged)))))

(event Custom|DEBUG_OnComboSelectionChanged
  (params (SelectedItem :type String) (SelectionType :type ESelectInfo%20Enum :default "OnKeyPress"))
  ;[1 0 0] [DEBUG] Testing debug stuff actually. Kindof interesting. If the debug stuff doesn't work, how do you debug that? Fuck.
  (Development|PrintString SelectedItem))

(event Custom|DEBUG_OnCheckboxStateChanged
  (params (bIsChecked :type Boolean))
  ;[1 0 0] [DEBUG] Testing debug stuff actually. Kindof interesting. If the debug stuff doesn't work, how do you debug that? Fuck.
  (Development|PrintString (Utilities|String|ToString(Boolean) bIsChecked)))

(event Input|ActionEvents|InputActionTestInput
  (params (Key :type Key%20Structure))
  (:Pressed
    (Class|MandaUtilitiesLibrary|PrintStringtoChannel (Utilities|GetDisplayName (Pawn|GetControlledPawn)) 7777)
    (AI|Navigation|SimpleMovetoLocation self (Math|Vector|MakeVector 0.0 0.0 0.0))))

(fn ConstructionScript)

(fn MandaPlayer
  (bind _asbp_manda_player_new (Utilities|Casting|CastToBP_MandaPlayerNew (Pawn|GetControlledPawn)))
  (return _asbp_manda_player_new))