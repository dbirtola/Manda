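; Player inventory component that holds the player's owned items in a single array.
; It supports adding items, removing a given or last item, clearing, counting, and looking items up by exact class, singly or as a required set.
; Removals send each affected item a remove message, and every add, remove or clear fires an InventoryUpdated notification.
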(fn ClearInventory
  (for _array_element (Variables|Default|GetOwnedItems)
    (Class|BPIInteractable|Remove(Message) _array_element (Components|GetOwner)))
  (Utilities|Array|Clear (Variables|Default|GetOwnedItems))
  (Default|CallInventoryUpdated))

(fn HasItem
  (params (Item%20Class :type BP%20Collectable%20Class%20Reference%20%28by%20ref%29))
  (for _array_element (Variables|Default|GetOwnedItems)
    (if (== (Utilities|GetClass _array_element) Item%20Class)
      (return _array_element)))
  (return 0))

(fn RemoveLast
  (bind _owneditems (Variables|Default|GetOwnedItems))
  (bind _owneditems_2 (Variables|Default|GetOwnedItems))
  (bind _returnvalue (Utilities|Array|Length _owneditems))
  (bind _returnvalue_2 (- _returnvalue 1))
  (bind _output (Utilities|Array|Get(acopy) _owneditems_2 _returnvalue_2))
  (Utilities|Array|RemoveIndex _owneditems _returnvalue_2)
  (Class|BPIInteractable|Remove(Message) _output (Components|GetOwner))
  (Default|CallInventoryUpdated)
  (return _output))

(fn AddItem
  (params (Item :type BP%20Collectable%20Object%20Reference))
  (Utilities|Array|Add (Variables|Default|GetOwnedItems) Item)
  (Default|CallInventoryUpdated))

(fn RemoveItem
  (params (ItemToRemove :type BP%20Collectable%20Object%20Reference))
  (Utilities|ArrayContains (Variables|Default|GetOwnedItems) ItemToRemove
    (:Yes
      (Utilities|Array|RemoveItem (Variables|Default|GetOwnedItems) ItemToRemove)
      (Class|BPIInteractable|Remove(Message) ItemToRemove)
      (Default|CallInventoryUpdated))))

(fn HasAllItems
  (params (ClassesToCheck :type Array%20of%20BP%20Collectable%20Class%20References))
  (for _array_element ClassesToCheck
    (bind _returnvalue (CallFunction|HasItem _array_element))
    (Utilities|IsValid _returnvalue
      (:Is%20Not%20Valid
        (return false))))
  (return true))

(fn GetNumItems
  (return (Utilities|Array|Length (Variables|Default|GetOwnedItems))))