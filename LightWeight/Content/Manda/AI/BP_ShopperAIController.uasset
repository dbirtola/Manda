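; AI controller for BP_Shopper that hunts alcohol pickups and runs from players once carrying any.
; A looping half-second timer caches the nearest BP_Alcohol as ClosestCollectable.
; Each Tick moves the shopper toward that target or, when alcohol is attached, a short step directly away from the closest BP_MandaPlayerNew.
; Victim-chasing logic, with dashes at item-carrying players or shoppers, is present but disconnected.
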(event EventBeginPlay
  ;[1 1 1] Get Controlled Shopper
  (bind _asbp_shopper (Utilities|Casting|CastToBP_Shopper (Pawn|GetControlledPawn))
    (:then
      (Variables|Default|SetShopper _asbp_shopper))
    (:CastFailed
      _))
  (CallFunction|UpdateClosestVariables)
  (Utilities|Time|SetTimerbyFunctionName 0 "UpdateClosestVariables" 0.5 true))

(event EventTick
  (params (DeltaSeconds :type Float%20%28single-precision%29))
  (bind _closestcollectable (Variables|Default|GetClosestCollectable))
  (bind _returnvalue (Utilities|IsValid _closestcollectable))
  (Utilities|IsValid (Variables|Default|GetShopper)
    (:Is%20Valid
      (if (> (Utilities|Array|Length (Variables|/Game/Manda/AI/BP_Shopper.BP_Shopper_C|GetAttachedAlcohol (Variables|Default|GetShopper))) 0)
        (bind _outactors (Actor|GetAllActorsOfClass "/Game/Manda/Player/BP_MandaPlayerNew.BP_MandaPlayerNew_C"))
        (bind _closestactorfound (CallFunction|FindClosestActor _outactors))
        (Utilities|IsValid _closestactorfound
          (:Is%20Valid
            (Default|MovetoLocation (Variables|Default|GetShopper) (+ (* (Math|Vector|Normalize (- (Transformation|GetActorLocation (Pawn|GetControlledPawn)) (Transformation|GetActorLocation _closestactorfound))) 1.5e+02) (Transformation|GetActorLocation (Pawn|GetControlledPawn))))))
        (elif _returnvalue
          (if _returnvalue
            (Default|Moveto (Variables|Default|GetShopper) (Variables|Default|GetClosestCollectable))))))))

(fn ConstructionScript)

(fn FindClosestCollectable
  (for _array_element (Variables|Default|GetCollectables)
    (if (> (LocalVariables|GetDistance) (Transformation|GetDistanceTo self _array_element))
      (LocalVariables|SettempClosestCollectable _array_element)
      (LocalVariables|SetDistance (Transformation|GetDistanceTo self _array_element))))
  (return (LocalVariables|GettempClosestCollectable)))

(fn UpdateCollectablesList
  (Utilities|Array|Clear (Variables|Default|GetCollectables))
  (bind _outactors (Actor|GetAllActorsOfClass "/Game/Manda/Collectables/BP_Alcohol.BP_Alcohol_C"))
  (for _array_element _outactors
    (Utilities|Array|Add (Variables|Default|GetCollectables) _array_element)))

(fn FindClosestVictim
  (for _array_element (Variables|Default|GetVictims)
    (Utilities|IsValid (Actor|GetComponentbyClass _array_element "/Game/Manda/Player/BPC_PlayerInventory.BPC_PlayerInventory_C")
      (:Is%20Valid
        (bind _numitems (Default|GetNumItems (Actor|GetComponentbyClass _array_element "/Game/Manda/Player/BPC_PlayerInventory.BPC_PlayerInventory_C")))
        (if (and (> _numitems 0) (< (Transformation|GetDistanceTo (Pawn|GetControlledPawn) _array_element) (LocalVariables|GetDistance)))
          (LocalVariables|SettempClosestVictim _array_element)
          (LocalVariables|SetDistance (Transformation|GetDistanceTo (Pawn|GetControlledPawn) _array_element))))))
  (return (LocalVariables|GettempClosestVictim)))

(fn FindClosestActor
  (params (ActorsToSearch :type Array%20of%20Actor%20Object%20References))
  (for _array_element ActorsToSearch
    (if (> (LocalVariables|GetDistance) (Transformation|GetDistanceTo self _array_element))
      (LocalVariables|SetDistance (Transformation|GetDistanceTo self _array_element))
      (LocalVariables|SetClosestActor _array_element)))
  (return (LocalVariables|GetClosestActor)))

(fn UpdateClosestVariables
  ;[1 1 1] Get All Collectables
  (Utilities|Array|Clear (Variables|Default|GetCollectables))
  (bind _outactors (Actor|GetAllActorsOfClass "/Game/Manda/Collectables/BP_Alcohol.BP_Alcohol_C"))
  (Utilities|Array|AppendArray (Variables|Default|GetCollectables) _outactors)
  (bind _closestcollectablefound (CallFunction|FindClosestCollectable))
  (Variables|Default|SetClosestCollectable _closestcollectablefound))