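; Chips prop that plays bottle clank sounds at the impact point when hit.
; The Hit event compares the hit location's vector length (not impact force) to a threshold: above plays BottleClank02, otherwise BottleClank01.
; Volume scales with the actor's X velocity and is clamped.
; Each sound has a DoOnce gate reset after a short delay to limit repeats.
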(event Collision|EventHit
  (params (MyComp :type Primitive%20Component%20Object%20Reference) (Other :type Actor%20Object%20Reference) (OtherComp :type Primitive%20Component%20Object%20Reference) (bSelfMoved :type Boolean) (HitLocation :type Vector :default "0, 0, 0") (HitNormal :type Vector :default "0, 0, 0") (NormalImpulse :type Vector :default "0, 0, 0") (Hit :type Hit%20Result%20Structure%20%28by%20ref%29))
  (bind _returnvalue (Transformation|GetVelocity))
  (bind _x (Math|Vector|BreakVector _returnvalue))
  (bind _returnvalue_2 (Math|Conversions|ToVector(Float) _x))
  (bind _returnvalue_3 (Math|Vector|VectorLength _returnvalue_2))
  (bind _returnvalue_4 (/ _returnvalue_3 1.5e+02))
  (bind _returnvalue_5 (Math|Float|Clamp(Float) _returnvalue_4 0.0 1.4))
  (Math|Float|CompareFloat (Math|Vector|VectorLength HitLocation) 3e+03
    (:>
      (Utilities|FlowControl|DoOnce false :!label _label
        (:Completed
          (Audio|PlaySoundatLocation "/Game/Manda/Audio/bottleClank02.bottleClank02" HitLocation "0, 0, 0" _returnvalue_5 1.0 0.0 0 0 0)
          (Utilities|FlowControl|Delay 0.2)
          (goto _label Reset))))
    (:==
      _)
    (:<
      _))
  (Utilities|FlowControl|DoOnce false :!label _label_2
    (:Completed
      (Audio|PlaySoundatLocation "/Game/Manda/Audio/bottleClank01.bottleClank01" HitLocation "0, 0, 0" _returnvalue_5 1.0 0.0 0 0 0)
      (Utilities|FlowControl|Delay 0.3)
      (goto _label_2 Reset))))

(fn ConstructionScript)