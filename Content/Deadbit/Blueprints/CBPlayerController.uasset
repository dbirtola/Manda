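; Player controller that holds the player's robot team, owned parts and known code pieces, and spawns the Bits actor at start.
; Recruiting respects a team size cap and scales robot max health, while dispatchers broadcast team, part and code-piece changes.
; Interact uses the pawn's overlap collider, opening a selection popup when several robots overlap.
; It also opens robot inspector and editor HUDs, and binds save, tutorial and debug health/damage keys.
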(event Custom|Edit%20Robot
  (params (Robot :type Modular%20Robot%20Object%20Reference))
  (Default|ToggleRobotEditor (Variables|Default|GetHUD) Robot))

(event Custom|Inspect%20Robot
  (params (Robot :type Modular%20Robot%20Object%20Reference))
  (Default|ToggleRobotInspector (Variables|Default|GetHUD) Robot)
  (Pawn|Components|CharacterMovement|DisableMovement (Variables|/Script/Engine.Character|GetCharacterMovement (.AsPlayer%20Character (Utilities|Casting|CastToPlayerCharacter (Pawn|GetControlledPawn))))))

(event Custom|AddRobot
  (params (Robot :type Modular%20Robot%20Object%20Reference))
  (bind _widget (Variables|/Game/Deadbit/Blueprints/RobotParts/ModularRobot.ModularRobot_C|GetWidget Robot))
  (bind _health (Variables|/Game/Deadbit/Blueprints/RobotParts/ModularRobot.ModularRobot_C|GetHealth Robot))
  (bind _asegg_bot (Utilities|Casting|CastToEggBot Robot)
    (:then
      (Default|SetCombatVisualState _asegg_bot false))
    (:CastFailed
      _))
  (Variables|/Game/Deadbit/Blueprints/Health/Health.Health_C|SetmaxHealth _health (* (Variables|/Game/Deadbit/Blueprints/Health/Health.Health_C|GetmaxHealth _health) (Variables|Default|GetPlayer%20Robot%20Health%20Multiplier)))
  (Physics|SetSimulatePhysics (Variables|/Game/Deadbit/Blueprints/RobotParts/ModularRobot.ModularRobot_C|GetCapsule Robot) false)
  (Utilities|Array|Add (Variables|Default|GetOwnedRobots) Robot)
  (Default|AssignOwnership Robot (Pawn|GetControlledPawn))
  (Default|CallTeamModified (Variables|Default|GetOwnedRobots))
  (Default|CallRobotRecruited Robot)
  (Rendering|SetVisibility _widget true true)
  (bind _asrobot_health_bar (Utilities|Casting|CastToRobotHealthBar (UserInterface|GetUserWidgetObject _widget))
    (:then
      (Default|SetAlly _asrobot_health_bar true))
    (:CastFailed
      _))
  (EventDispatchers|BindEventtoRobotModified Robot (delegate Custom|RobotModified))
  (EventDispatchers|AssignDeath (Variables|/Game/Deadbit/Blueprints/RobotParts/ModularRobot.ModularRobot_C|GetHealth Robot) (delegate Custom|RemoveBot)))

(event Custom|OnRobotModified
  (params (Robot :type Modular%20Robot%20Object%20Reference))
  (Default|CallTeamModified (Variables|Default|GetOwnedRobots)))

(event Custom|RemoveBot
  (bind _ownedrobots (Variables|Default|GetOwnedRobots))
  (bind _output (Utilities|Array|Get(acopy) _ownedrobots))
  (bind _health (Variables|/Game/Deadbit/Blueprints/RobotParts/ModularRobot.ModularRobot_C|GetHealth _output))
  (Utilities|IsValid _output
    (:Is%20Valid
      (Variables|/Game/Deadbit/Blueprints/Health/Health.Health_C|SetmaxHealth _health (/ (Variables|/Game/Deadbit/Blueprints/Health/Health.Health_C|GetmaxHealth _health) (Variables|Default|GetPlayer%20Robot%20Health%20Multiplier)))
      (Default|AssignOwnership _output)
      (bind _alive (Default|IsAlive (Variables|/Game/Deadbit/Blueprints/RobotParts/ModularRobot.ModularRobot_C|GetHealth _output)))
      (if _alive
        (Default|TakeDamage (Variables|/Game/Deadbit/Blueprints/RobotParts/ModularRobot.ModularRobot_C|GetHealth _output) 5e+03)
        (else
          (Utilities|Array|RemoveItem (Variables|Default|GetOwnedRobots) _output)
          (Default|CallTeamModified (Variables|Default|GetOwnedRobots)))))))

(event Custom|Option%20Selected
  (params (Option :type String) (Object :type Object%20Object%20Reference))
  ;[1 1 1] Interact with object in front of player
  (bind _asmodular_robot (Utilities|Casting|CastToModularRobot Object))
  (Default|Interact _asmodular_robot self))

(event Custom|RobotModified
  (params (Robot :type Modular%20Robot%20Object%20Reference) (BodyPart :type Robot%20Part%20Object%20Reference))
  (Default|CallTeamModified (Variables|Default|GetOwnedRobots)))

(event Custom|AddAvailablePiece
  (params (New%20Piece :type Code%20Piece%20Class%20Reference))
  (Utilities|Array|AddUnique (Variables|Default|GetKnownCodePieces) New%20Piece))

(event Custom|AddCodePieces
  (params (Code%20Pieces :type Array%20of%20Code%20Piece%20Class%20References) (Notify%20Player :type Boolean))
  (for _array_element Code%20Pieces
    (Utilities|Array|AddUnique (Variables|Default|GetKnownCodePieces) _array_element))
  (Default|CallCodePiecesAdded Code%20Pieces Notify%20Player))

(event EventBeginPlay
  (bind _returnvalue (Pawn|GetControlledPawn))
  (Development|ExecuteConsoleCommand "DisableAllScreenMessages" 0)
  (Utilities|FlowControl|Delay 0.2)
  (bind _returnvalue_2 (Game|SpawnActorfromClass "/Game/Deadbit/Blueprints/JustBits/Bits_BP.Bits_BP_C" (Math|Transform|MakeTransform (+ (Transformation|GetActorLocation _returnvalue) "-20.000000, 0,0.000000") "0, 0, 0" "1,1,1") "AlwaysSpawn" _returnvalue _returnvalue))
  (Variables|Default|SetBits _returnvalue_2))

(event Input|KeyboardEvents|L
  (params (Key :type Key%20Structure))
  (:Pressed
    (Development|PrintString "Hello")))

(event Input|KeyboardEvents|Q
  (params (Key :type Key%20Structure))
  (:Pressed
    (Default|ContinueTutorial (Variables|Default|GetHUD))))

(event Input|KeyboardEvents|N
  (params (Key :type Key%20Structure))
  (:Pressed
    (Default|TakeDamage (Variables|/Game/Deadbit/Blueprints/ThirdPersonCharacter/PlayerCharacter.PlayerCharacter_C|GetHealth (.AsPlayer%20Character (Utilities|Casting|CastToPlayerCharacter (Pawn|GetControlledPawn)))) 1e+04)))

(event Input|KeyboardEvents|E
  (params (Key :type Key%20Structure))
  (bind _returnvalue (Pawn|GetControlledPawn))
  (bind _asplayer_character (Utilities|Casting|CastToPlayerCharacter _returnvalue))
  (bind _interactioncollider (Variables|/Game/Deadbit/Blueprints/ThirdPersonCharacter/PlayerCharacter.PlayerCharacter_C|GetInteractionCollider _asplayer_character))
  (bind _overlappingactors (Collision|GetOverlappingActors _interactioncollider "/Script/Engine.Actor" :!class /Script/Engine.PrimitiveComponent))
  ;[1 1 1] Interact with object in front of player
  (:Pressed
    (bind _filteredarray (Utilities|Array|FilterArray _overlappingactors "/Game/Deadbit/Blueprints/RobotParts/ModularRobot.ModularRobot_C"))
    (if (>= (Utilities|Array|Length _filteredarray) 2)
      (Utilities|Array|Clear (Variables|Default|GetRobot%20Selection%20Array))
      (Utilities|Array|Clear (Variables|Default|GetRobot%20Selections))
      (for _array_element _filteredarray
        (bind _asmodular_robot (Utilities|Casting|CastToModularRobot _array_element))
        (Utilities|Array|Add (Variables|Default|GetRobot%20Selection%20Array) (Variables|/Game/Deadbit/Blueprints/RobotParts/ModularRobot.ModularRobot_C|GetRobotName _asmodular_robot))
        (Utilities|Array|Add (Variables|Default|GetRobot%20Selections) _asmodular_robot))
      (bind _returnvalue_2 (UserInterface|CreateWidget "/Game/Deadbit/Blueprints/UI/SelectionPopup.SelectionPopup_C"))
      (UserInterface|Viewport|AddtoViewport _returnvalue_2 50)
      (Default|RequestSelection _returnvalue_2 "" (Variables|Default|GetRobot%20Selection%20Array) (Variables|Default|GetRobot%20Selections))
      (EventDispatchers|BindEventtoOptionSelected _returnvalue_2 (delegate Custom|Option%20Selected))
      (else
        (bind _array_element_2 (Utilities|Array|ForEachLoopwithBreak _overlappingactors :!label _label)
          (:LoopBody
            (bind _success (Class|IInteractable|Interact(Message) _array_element_2 self))
            (if _success
              (goto _label Break))))))))

(event Input|KeyboardEvents|M
  (params (Key :type Key%20Structure))
  (:Pressed
    (for _array_element (Collision|GetOverlappingActors (Variables|/Game/Deadbit/Blueprints/ThirdPersonCharacter/PlayerCharacter.PlayerCharacter_C|GetInteractionCollider (.AsPlayer%20Character (Utilities|Casting|CastToPlayerCharacter (Game|Player|GetPlayerPawn 0)))) 0 :!class /Script/Engine.PrimitiveComponent)
      (Utilities|Casting|CastToPlayerCharacter _array_element
        (:CastFailed
          (Game|Damage|ApplyDamage _array_element 2e+01 0 0))))))

(event Input|KeyboardEvents|V
  (params (Key :type Key%20Structure))
  (:Pressed
    (bind _outactors (Actor|GetAllActorsOfClass "/Game/Deadbit/Blueprints/GameManager.GameManager_C"))
    (Default|SaveGame (Utilities|Array|Get(acopy) _outactors))))

(event Input|KeyboardEvents|X
  (params (Key :type Key%20Structure)))

(event Input|KeyboardEvents|B
  (params (Key :type Key%20Structure))
  (:Pressed
    (bind _outactors (Actor|GetAllActorsOfClass "/Game/Deadbit/Blueprints/TutorialSteps/Groundwork/TutorialManager.TutorialManager_C"))
    (Default|SkipStep (Utilities|Array|Get(acopy) _outactors))))

(event Input|KeyboardEvents|Comma
  (params (Key :type Key%20Structure))
  (:Pressed
    (bind _asplayer_character (Utilities|Casting|CastToPlayerCharacter (Game|GetPlayerCharacter 0)))
    (Variables|/Game/Deadbit/Blueprints/Health/Health.Health_C|SetmaxHealth (Variables|/Game/Deadbit/Blueprints/ThirdPersonCharacter/PlayerCharacter.PlayerCharacter_C|GetHealth _asplayer_character) 3e+04)
    (Variables|/Game/Deadbit/Blueprints/Health/Health.Health_C|SetHealth (Variables|/Game/Deadbit/Blueprints/ThirdPersonCharacter/PlayerCharacter.PlayerCharacter_C|GetHealth _asplayer_character) 3e+04)))

(fn ConstructionScript)

(fn PickupPart
  (params (Part :type Robot%20Part%20Object%20Reference))
  (Utilities|Array|Add (Variables|Default|GetOwnedParts) Part)
  (Audio|PlaySound2D "/Game/Deadbit/Sound/SoundCues/PickupItem.PickupItem" 1.0 1.0 0.0 0 0)
  (Default|CallPartsListModified (Variables|Default|GetOwnedParts)))

(fn RemovePart
  (params (Robot%20Part :type Robot%20Part%20Object%20Reference))
  (Utilities|Array|RemoveItem (Variables|Default|GetOwnedParts) Robot%20Part)
  (Default|CallPartsListModified (Variables|Default|GetOwnedParts)))

(fn GetNearestRobottoPlayer
  (bind _returnvalue (Pawn|GetControlledPawn))
  (bind _outactors (Actor|GetAllActorsOfClass "/Game/Deadbit/Blueprints/RobotParts/ModularRobot.ModularRobot_C"))
  (LocalVariables|SetClosest%20So%20Far (Utilities|Array|Get(acopy) _outactors))
  (for _array_element _outactors
    (if (< (Transformation|GetDistanceTo _array_element _returnvalue) (Transformation|GetDistanceTo _returnvalue (LocalVariables|GetClosest%20So%20Far)))
      (LocalVariables|SetClosest%20So%20Far _array_element)))
  (return (.AsModular%20Robot (Utilities|Casting|CastToModularRobot (LocalVariables|GetClosest%20So%20Far)))))

(fn GetAvailableCodePieces
  (for _array_element (Variables|Default|GetOwnedRobots)
    (Utilities|FlowControl|Sequence
      (:then_0
        (bind _code_pieces (Default|GetAvailableCodePieces _array_element))
        (for _array_element_2 _code_pieces
          (Utilities|Array|AddUnique (Variables|Default|GetKnownCodePieces) _array_element_2)))
      (:then_1
        (bind _keys (Utilities|Map|Keys (Variables|/Game/Deadbit/Blueprints/RobotParts/ModularRobot.ModularRobot_C|GetEquippedParts _array_element)))
        (for _array_element_3 _keys
          (Utilities|IsValid (.Value (Utilities|Map|Find (Variables|/Game/Deadbit/Blueprints/RobotParts/ModularRobot.ModularRobot_C|GetEquippedParts _array_element) _array_element_3))
            (:Is%20Valid
              (for _array_element_4 (Variables|/Game/Deadbit/Blueprints/RobotParts/RobotPart.RobotPart_C|GetGrantedCodePieces (.Value (Utilities|Map|Find (Variables|/Game/Deadbit/Blueprints/RobotParts/ModularRobot.ModularRobot_C|GetEquippedParts _array_element) _array_element_3)))
                (Utilities|Array|AddUnique (Variables|Default|GetKnownCodePieces) _array_element_4))))))))
  (for _array_element_5 (Variables|Default|GetOwnedParts)
    (for _array_element_6 (Variables|/Game/Deadbit/Blueprints/RobotParts/RobotPart.RobotPart_C|GetGrantedCodePieces _array_element_5)
      (Utilities|Array|AddUnique (Variables|Default|GetKnownCodePieces) _array_element_6)))
  (return (Variables|Default|GetKnownCodePieces)))

(fn LearnCodePiece
  (params (Code%20Piece :type Code%20Piece%20Object%20Reference))
  (bind _returnvalue (Utilities|GetClass Code%20Piece))
  (bind _newparam (CallFunction|GetAvailableCodePieces))
  (if (not (Utilities|Array|ContainsItem _newparam _returnvalue))
    (Utilities|Array|Add (Variables|Default|GetKnownCodePieces) _returnvalue)))

(fn RecruitRobot
  (params (Modular%20Robot :type Modular%20Robot%20Object%20Reference))
  (if (< (Utilities|Array|Length (Variables|Default|GetOwnedRobots)) (Variables|Default|GetMaximumTeamSize))
    (CallFunction|AddRobot Modular%20Robot)
    (Default|Revive Modular%20Robot 1.0)
    (else
      (Default|CallActionFailed "NewEnumerator0" Modular%20Robot))))