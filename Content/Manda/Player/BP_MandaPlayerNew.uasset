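; Player pawn for a physics-driven, wobbly character whose handling changes with a drunk level, adjustable by debug inputs.
; Input pushes a sphere relative to camera yaw, skewed by Perlin noise, while the root follows it.
; Body lean feeds the forward push and an upward righting force at the head, and limits speed.
; Curves map drunk level to those forces, sphere mass, noise range and top speed; overlaps trigger pickups when allowed.
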(event EventDebugIncrease
  (CallFunction|ApplyDrunkLevel (+ (Variables|Default|GetDrunkLevel) 1.0))
  (Class|MandaUtilitiesLibrary|PrintStringtoChannel (Utilities|String|Append "DRUNK LEVEL: " (Utilities|String|ToString(Float) (Variables|Default|GetDrunkLevel))) 7777 true true "(R=1.000000,G=0.221514,B=0.000000,A=1.000000)"))

(event EventDebugDecrease
  (CallFunction|ApplyDrunkLevel (+ (Variables|Default|GetDrunkLevel) -1.0))
  (Class|MandaUtilitiesLibrary|PrintStringtoChannel (Utilities|String|Append "DRUNK LEVEL: " (Utilities|String|ToString(Float) (Variables|Default|GetDrunkLevel))) 7777 true true "(R=1.000000,G=0.221514,B=0.000000,A=1.000000)"))

(event EventMoveForward
  (params (Value :type Float%20%28single-precision%29))
  (bind _returnvalue (Utilities|BodyUpAxis))
  (bind _returnvalue_2 (* _returnvalue 5e+03))
  (bind _hor (CallFunction|HorizontalVector _returnvalue_2))
  (Variables|Default|SetForwardInput Value)
  (Physics|AddForce (Variables|Default|GetSphere) (+ (* (Math|Vector|RotateVector (Math|Vector|MakeVector 1e+04 0.0 0.0) (Utilities|ZRotation)) (Variables|Default|GetForwardInput)) (Math|Vector|MakeVector (.x _hor) (.y _hor) 0.0)) "None" false))

(event EventMoveRight
  (params (Value :type Float%20%28single-precision%29))
  (Variables|Default|SetRightInput Value)
  (Physics|AddForce (Variables|Default|GetSphere) (* (Math|Vector|RotateVector (Math|Vector|MakeVector 0.0 1e+04 0.0) (Utilities|ZRotation)) (Variables|Default|GetRightInput)) "None" false))

(event EventBeginPlay
  (CallFunction|ApplyDrunkLevel 0.0))

(event Collision|EventActorBeginOverlap
  (params (OtherActor :type Actor%20Object%20Reference))
  (if (Variables|Default|GetbCanPickUpItems)
    (Class|BPIInteractable|Interact(Message) OtherActor self)))

(event EventTurnRight
  (params (Value :type Float%20%28single-precision%29))
  (Transformation|AddWorldRotation (Variables|Default|GetSpringArm) (Math|Rotator|MakeRotator 0.0 0.0 Value) false false))

(event EventTurnUp
  (params (Value :type Float%20%28single-precision%29))
  (Transformation|AddLocalRotation (Variables|Default|GetSpringArm) (Math|Rotator|MakeRotator 0.0 Value 0.0) false false))

(event EventTick
  (params (DeltaSeconds :type Float%20%28single-precision%29))
  (bind _returnvalue (Utilities|BodyUpAxis))
  (bind _hor (CallFunction|HorizontalVector _returnvalue))
  (Transformation|SetWorldLocation (Variables|Default|GetDefaultSceneRoot) (Transformation|GetWorldLocation (Variables|Default|GetSphere)) false false)
  (Class|PrimitiveComponent|AddForceatLocation (Variables|Default|GetCube2) (Math|Vector|MakeVector 0.0 0.0 (+ (* (Math|Vector2D|Vector2DLength (+ _hor (* (Utilities|RotatedMovementInput) (Math|Vector2D|Vector2DLength _hor)))) (Variables|Default|GetUpDraft)) (Variables|Default|GetConstant%20Up))) (Transformation|GetWorldLocation (Variables|Default|GetHeadBone)) "None")
  (Physics|SetPhysicsLinearVelocity (Variables|Default|GetSphere) (Math|Vector|ClampVectorSize (Transformation|GetComponentVelocity (Variables|Default|GetSphere)) 0.0 (* (Variables|Default|GetMaxSpeed) (Math|Float|Square (Math|Float|Max(Float) (.z (Utilities|BodyUpAxis)) 0.0)))) false "None"))

(fn ConstructionScript)

(fn GetHorizontalVelocity
  (params (Target :type Scene%20Component%20Object%20Reference))
  (bind _returnvalue (Transformation|GetComponentVelocity Target))
  (return (Math|Vector2D|MakeVector2D (.x _returnvalue) (.y _returnvalue))))

(fn HorizontalVector
  (params (Vector :type Vector))
  (return (Math|Vector2D|MakeVector2D (.x Vector) (.y Vector))))

(fn ApplyDrunkLevel
  (params (Level :type Float%20%28single-precision%29))
  (Variables|Default|SetDrunkLevel Level)
  (Variables|Default|SetUpDraft (Math|Curves|GetFloatValue (Variables|Curves|GetCorrectiveForceCurve) Level))
  (Class|PrimitiveComponent|SetMassScale (Variables|Default|GetSphere) "None" (Math|Curves|GetFloatValue (Variables|Curves|GetFrictionCurve) Level))
  (Variables|Default|SetConstant%20Up (Math|Curves|GetFloatValue (Variables|Curves|GetConstantUpCurve) Level))
  (Variables|Default|SetAngleOffsetRange (Math|Curves|GetFloatValue (Variables|Curves|GetAngleOffsetCurve) Level))
  (Variables|Default|SetMaxSpeed (Math|Curves|GetFloatValue (Variables|Curves|GetMaxSpeedCurve) Level)))