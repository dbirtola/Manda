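; BP_MandaPlayerTemp is a temporary player pawn for Manda with basic axis-driven movement and turning.
; Forward and right inputs rotate fixed vectors by ZRotation and feed them to the movement component from MandaMovement, printing debug values to channels.
; Turn input yaws the SpringArm in world space.
; The ZRotation and MandaMovement helpers contain only unused nodes, with ZRotation's reading camera Roll rather than Yaw despite its name.
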(event Custom|MoveRight
  (params (Value :type Float%20%28single-precision%29))
  (bind _returnvalue (Math|Vector|MakeVector 0.0 1e+02 0.0))
  (bind _returnvalue_2 (Utilities|ZRotation))
  (bind _returnvalue_3 (Math|Vector|RotateVector _returnvalue _returnvalue_2))
  (bind _returnvalue_4 (* _returnvalue_3 Value))
  (Class|MandaUtilitiesLibrary|PrintStringtoChannel (Utilities|String|ToString(Vector) _returnvalue_4) 101 true true "(R=1.000000,G=0.767847,B=0.000000,A=1.000000)")
  (Class|PawnMovementComponent|AddInputVector (Utilities|MandaMovement) _returnvalue_4 false))

(event Custom|MoveForward
  (params (Value :type Float%20%28single-precision%29))
  (bind _returnvalue (Utilities|ZRotation))
  (Class|MandaUtilitiesLibrary|PrintStringtoChannel (Utilities|String|ToString(Rotator) _returnvalue) 100 true true "(R=0.045007,G=1.000000,B=0.000000,A=1.000000)")
  (Class|PawnMovementComponent|AddInputVector (Utilities|MandaMovement) (* (Math|Vector|RotateVector (Math|Vector|MakeVector 1e+02 0.0 0.0) _returnvalue) Value) false))

(event Custom|RotateTurnRight
  (params (Value :type Float%20%28single-precision%29))
  (Transformation|AddWorldRotation (Variables|Default|GetSpringArm) (Math|Rotator|MakeRotator 0.0 0.0 Value) false false))

(fn ConstructionScript)