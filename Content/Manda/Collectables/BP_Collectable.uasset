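; BP_Collectable is a physics-driven pickup actor that can be stored in and removed from the player's inventory.
; Interact hides the mesh, stops physics, moves the actor to the world origin and adds it to the instigator's BPC_PlayerInventory component.
; Remove reverses this, placing the actor at the instigator's location with visibility and physics restored and a small upward impulse.
; The same actor instance is parked rather than destroyed while stored.
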(event EventInteract
  (params (Instigator :type Actor%20Object%20Reference))
  (bind _mesh (Variables|Default|GetMesh))
  (Rendering|SetVisibility _mesh false true)
  (Physics|SetSimulatePhysics _mesh false)
  (Transformation|SetActorLocation "0, 0, 0" false false)
  (Default|AddItem (Actor|GetComponentbyClass Instigator "/Game/Manda/Player/BPC_PlayerInventory.BPC_PlayerInventory_C") self))

(event EventRemove
  (params (Instigator :type Actor%20Object%20Reference))
  (bind _mesh (Variables|Default|GetMesh))
  (Rendering|SetVisibility _mesh true true)
  (Physics|SetSimulatePhysics _mesh true)
  (Transformation|SetActorLocation (Transformation|GetActorLocation Instigator) false false)
  (Physics|AddImpulse (Variables|Default|GetMesh) "0, 0,100.000000" "None" false))

(fn ConstructionScript)