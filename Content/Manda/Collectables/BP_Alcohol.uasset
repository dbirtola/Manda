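; BP_Alcohol is a collectable pickup that sends a DrunkUp message to whoever interacts with it.
; Collect, Interact and Remove call the parent collectable logic, with Interact then adding the drunk message.
; BeginPlay tilts the mesh and gives it a random yaw.
; Tick spins it on both world and local yaw and bobs it by adding a time-based sine to its height each frame, so bob amplitude depends on frame rate.
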(event EventCollect
  (|CallParentFunction))

(event EventTick
  (params (DeltaSeconds :type Float%20%28single-precision%29))
  (bind _mesh (Variables|Character|GetMesh))
  (Transformation|SetRelativeLocation _mesh (+ (Variables|/Script/Engine.SceneComponent|GetRelativeLocation _mesh) (Math|Vector|MakeVector 0.0 0.0 (Math|Trig|Sin(Degrees) (* (Utilities|Time|GetGameTimeinSeconds) 1e+02)))) false false)
  (Transformation|AddWorldRotation (Variables|Character|GetMesh) (Math|Rotator|MakeRotator 0.0 0.0 (* (Utilities|Time|GetWorldDeltaSeconds) 1e+02)) false false)
  (Transformation|AddLocalRotation (Variables|Character|GetMesh) (Math|Rotator|MakeRotator 0.0 0.0 (* (Utilities|Time|GetWorldDeltaSeconds) 153.0)) false false))

(event EventInteract
  (params (Instigator :type Actor%20Object%20Reference))
  (|CallParentFunction Instigator)
  (Class|BPMandaInputInterface|DrunkUp(Message) Instigator))

(event EventBeginPlay
  (Transformation|AddWorldRotation (Variables|Character|GetMesh) (Math|Rotator|MakeRotator 3e+01 0.0 (* (Math|Random|RandomFloat) 3.6e+02)) false false))

(event EventRemove
  (params (Instigator :type Actor%20Object%20Reference))
  (|CallParentFunction Instigator))

(fn ConstructionScript
  (|CallParentFunction))