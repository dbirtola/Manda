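; Game mode for Manda that manages the round lifecycle: starting, retrying, ending and resetting.
; StartRound calls ResetLevel and then stores the given round info, while StartNextRound and RetryRound both pass it the current round info unchanged.
; EndRound broadcasts OnRoundEnded with the reason and a victory flag derived from it.
; A separate ResetMandaLevel event reloads the current level by name.
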(event Custom|End%20Round
  (params (Reason :type EEndRoundReason%20Enum :default "NewEnumerator0"))
  ;[1 1 1] End the current round
  (Default|CallOnRoundEnded (Utilities|Enum|Equal(Enum) Reason "NewEnumerator1") Reason))

(event Custom|Start%20Round
  (params (Round%20Info :type Round%20Info%20Structure))
  ;[1 1 1] Start a specific round
  (Class|GameModeBase|ResetLevel)
  (Variables|Default|SetCurrent%20Round%20Info Round%20Info))

(event Custom|Reset%20Manda%20Level
  ;[1 1 1] Reset the current level in preparation of starting a new round
  (bind _returnvalue (Game|GetCurrentLevelName true))
  (Game|OpenLevel(byName) (Utilities|String|StringToName _returnvalue)))

(event Custom|Retry%20Round
  ;[1 1 1] Retry the current round
  (CallFunction|StartRound (Variables|Default|GetCurrent%20Round%20Info)))

(event Custom|Start%20Next%20Round
  ;[1 1 1] Determines and starts the next round
  (CallFunction|StartRound (Variables|Default|GetCurrent%20Round%20Info)))

(fn ConstructionScript)