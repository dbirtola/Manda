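; BP_GroceryList builds a randomized list of collectables to serve as the required items of a grocery list.
; GenerateList clears RequiredCollectables, fills it with the requested number of picks from GetRandomCollectable, and returns it.
; Each pick independently indexes PossibleCollectables at random, so duplicates can occur.
; RandomInteger receives the array length minus one as its exclusive maximum, so the last entry is never picked when several exist.
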(fn GenerateList
  (params (List%20Length :type Integer))
  (Utilities|Array|Clear (Variables|Default|GetRequired%20Collectables))
  (for _index (range 0 (- List%20Length 1))
    (bind _random_collectable (CallFunction|GetRandomCollectable))
    (Utilities|Array|Add (Variables|Default|GetRequired%20Collectables) _random_collectable))
  (return (Variables|Default|GetRequired%20Collectables)))

(fn GetRandomCollectable
  (return (Utilities|Array|Get(acopy) (Variables|Default|GetPossible%20Collectables) (Math|Random|RandomInteger (- (Utilities|Array|Length (Variables|Default|GetPossible%20Collectables)) 1)))))