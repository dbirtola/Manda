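; BP_MandaPlayerNew is the physics-driven drunk player, balancing an upper body over a rolling sphere.
; Stick input pushes the sphere and head with noise-skewed, camera-relative forces, while Tick adds upright lift, drives the sphere toward the lean and caps speed by uprightness.
; ApplyDrunkLevel reads curves to retune handling and updates post-process and audio controllers.
; A timer finds the nearest alcohol for a ground arrow, which Tick rotates toward it.
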(event Custom|GetArrowHeight
  (bind _defaultsceneroot (Variables|Default|GetDefaultSceneRoot))
  (bind _returnvalue (Transformation|GetWorldLocation _defaultsceneroot))
  (bind _outhit (Collision|LineTraceByChannel _returnvalue (- _returnvalue "0,0.000000,10000.000000") "TraceTypeQuery1" false 0 "None"))
  (Variables|Default|SetArrowHeight (+ (.Z (Math|Vector|BreakVector (.Location (Collision|BreakHitResult _outhit)))) 1.0)))

(event Custom|SetNearestAlcohol
  (bind _defaultsceneroot (Variables|Default|GetDefaultSceneRoot))
  (bind _widgetlocation (Variables|Default|GetWidgetLocation))
  (bind _returnvalue (Transformation|GetWorldLocation _defaultsceneroot))
  (bind _mandagamemode (Utilities|MandaGameMode)
    (:then
      (bind _outmesh (Default|GetNearestAlcohol _mandagamemode (Transformation|GetWorldLocation (Variables|Default|GetDefaultSceneRoot))))
      (bind _output_get (Variables|Default|SetClosestAlcohol _outmesh))
      (Utilities|IsValid _output_get
        (:Is%20Valid
          (Utilities|FlowControl|Gate true) ; enters at Open
        )
        (:Is%20Not%20Valid
          (Utilities|FlowControl|Sequence
            (:then_0
              (bind _newtrack_0 (Timeline|OpacityTimline PlayFromStart)
                (:Update
                  (Class|WidgetComponent|SetTintColorandOpacity (Variables|Default|GetWidget) (Utilities|Struct|MakeLinearColor 1.0 1.0 1.0 _newtrack_0)))))
            (:then_1
              (Utilities|FlowControl|Gate true) ; enters at Close
            )
            (:then_2
              (Utilities|Time|ClearandInvalidateTimerbyHandle (stale EventBeginPlay _returnvalue)))))))))

(event Custom|ShowFrameRate
  (Rendering|Components|TextRender|SetText (Variables|Default|GetFramerateText) (Utilities|Text|ToText(Float) (/ 1.0 (Utilities|Time|GetWorldDeltaSeconds)) "HalfToEven")))

(event EventDebugIncrease
  (CallFunction|ApplyDrunkLevel (+ (Variables|Default|GetDrunkLevel) 1.0))
  (Class|MandaUtilitiesLibrary|PrintStringtoChannel (Utilities|String|Append "DRUNK LEVEL: " (Utilities|String|ToString(Float) (Variables|Default|GetDrunkLevel))) 7777 true true "(R=1.000000,G=0.221514,B=0.000000,A=1.000000)"))

(event EventDrunkUp
  (CallFunction|ApplyDrunkLevel (+ (Variables|Default|GetDrunkLevel) 2.0))
  (Class|MandaUtilitiesLibrary|PrintStringtoChannel (Utilities|String|Append "DRUNK LEVEL: " (Utilities|String|ToString(Float) (Variables|Default|GetDrunkLevel))) 7777 true true "(R=1.000000,G=0.221514,B=0.000000,A=1.000000)"))

(event EventDebugDecrease
  (CallFunction|ApplyDrunkLevel (+ (Variables|Default|GetDrunkLevel) -1.0))
  (Class|MandaUtilitiesLibrary|PrintStringtoChannel (Utilities|String|Append "DRUNK LEVEL: " (Utilities|String|ToString(Float) (Variables|Default|GetDrunkLevel))) 7777 true true "(R=1.000000,G=0.221514,B=0.000000,A=1.000000)"))

(event EventMoveForward
  (params (Value :type Float%20%28single-precision%29))
  (bind _output_get (Variables|Default|SetForwardInput (Utilities|AdjustforDeltaTime (Math|Float|Clamp(Float) Value -1.0))))
  (Class|MandaUtilitiesLibrary|PrintStringtoChannel (Utilities|String|ToString(Float) _output_get) 3 true true "(R=1.000000,G=0.196708,B=0.000000,A=1.000000)")
  (Physics|AddForce (Variables|Default|GetSphere) (* (Math|Vector|RotateVector (Math|Vector|MakeVector (Variables|Default|GetRightStickForce) 0.0 0.0) (Utilities|ZRotationLeftStick)) (Variables|Default|GetForwardInput)) "None" false))

(event EventMoveRight
  (params (Value :type Float%20%28single-precision%29))
  (Variables|Default|SetRightInput (Utilities|AdjustforDeltaTime (Math|Float|Clamp(Float) Value -1.0)))
  (Physics|AddForce (Variables|Default|GetSphere) (* (Math|Vector|RotateVector (Math|Vector|MakeVector 0.0 (Variables|Default|GetRightStickForce) 0.0) (Utilities|ZRotationLeftStick)) (Variables|Default|GetRightInput)) "None" false))

(event EventBeginPlay
  (CallFunction|GetArrowHeight)
  (Utilities|FlowControl|Delay 0.0)
  (CallFunction|ApplyDrunkLevel 0.0)
  (CallFunction|SetNearestAlcohol)
  (bind _returnvalue (Utilities|Time|SetTimerbyEvent (delegate Custom|SetNearestAlcohol) 0.5 true)))

(event Collision|EventActorBeginOverlap
  (params (OtherActor :type Actor%20Object%20Reference))
  (if (Variables|Default|GetbCanPickUpItems)
    (Class|BPIInteractable|Interact(Message) OtherActor self)))

(event EventTurnRight
  (params (Value :type Float%20%28single-precision%29))
  (Class|PrimitiveComponent|AddForceatLocation (Variables|Default|GetCube2) (* (Math|Vector|RotateVector (Math|Vector|MakeVector 0.0 1e+02 0.0) (Utilities|ZRotationLeftStick)) (Math|Conversions|ToVector(Float) (Utilities|AdjustforDeltaTime Value))) (Transformation|GetWorldLocation (Variables|Default|GetHeadBone)) "None"))

(event EventTurnUp
  (params (Value :type Float%20%28single-precision%29))
  (Class|PrimitiveComponent|AddForceatLocation (Variables|Default|GetCube2) (* (Math|Vector|RotateVector (Math|Vector|MakeVector -1e+02 0.0 0.0) (Utilities|ZRotationLeftStick)) (Math|Conversions|ToVector(Float) (Utilities|AdjustforDeltaTime Value))) (Transformation|GetWorldLocation (Variables|Default|GetHeadBone)) "None"))

(event EventTick
  (params (DeltaSeconds :type Float%20%28single-precision%29))
  (bind _returnvalue (Utilities|BodyUpAxis))
  (bind _out (Utilities|AdjustforDeltaTime 1.0))
  (bind _returnvalue_2 (Utilities|BodyUpAxis))
  (bind _closestalcohol (Variables|Default|GetClosestAlcohol))
  (bind _defaultsceneroot (Variables|Default|GetDefaultSceneRoot))
  (bind _widgetlocation (Variables|Default|GetWidgetLocation))
  (bind _widgetlocation_2 (Variables|Default|GetWidgetLocation))
  (bind _returnvalue_3 (* _returnvalue 5e+03))
  (bind _hor (CallFunction|HorizontalVector _returnvalue_2))
  (bind _returnvalue_4 (Transformation|GetWorldLocation _widgetlocation))
  (bind _returnvalue_5 (Transformation|GetWorldLocation _closestalcohol))
  (bind _returnvalue_6 (Transformation|GetWorldLocation _defaultsceneroot))
  (bind _returnvalue_7 (* _returnvalue_3 _out))
  (bind _returnvalue_8 (- (Math|Vector2D|MakeVector2D (.x _returnvalue_5) (.y _returnvalue_5)) (Math|Vector2D|MakeVector2D (.x _returnvalue_6) (.y _returnvalue_6))))
  (bind _returnvalue_9 (Math|Vector2D|Normalize2D _returnvalue_8))
  (Transformation|SetWorldLocation (Variables|Default|GetDefaultSceneRoot) (Transformation|GetWorldLocation (Variables|Default|GetSphere)) false false)
  (Class|PrimitiveComponent|AddForceatLocation (Variables|Default|GetCube2) (Math|Vector|MakeVector 0.0 0.0 (* (+ (* (Math|Vector2D|Vector2DLength (+ _hor (* (Utilities|RotatedMovementInput) (Math|Vector2D|Vector2DLength _hor)))) (Variables|Default|GetUpDraft)) (Variables|Default|GetConstant%20Up)) (Utilities|TimeMultiplier))) (Transformation|GetWorldLocation (Variables|Default|GetHeadBone)) "None")
  (Physics|AddForce (Variables|Default|GetSphere) (Math|Vector|MakeVector (.x _returnvalue_7) (.y _returnvalue_7) 0.0) "None" false)
  (Physics|SetPhysicsLinearVelocity (Variables|Default|GetSphere) (Math|Vector|ClampVectorSize (Transformation|GetComponentVelocity (Variables|Default|GetSphere)) 0.0 (* (Variables|Default|GetMaxSpeed) (Math|Float|Square (Math|Float|Max(Float) (.z (Utilities|BodyUpAxis)) 0.0)))) false "None")
  (Transformation|SetWorldLocation _widgetlocation (Math|Vector|MakeVector (.x _returnvalue_4) (.y _returnvalue_4) (Variables|Default|GetArrowHeight)) false false)
  (Utilities|FlowControl|Gate true
    (:Exit
      (Transformation|SetWorldRotation _widgetlocation_2 (Math|Rotator|Lerp(Rotator) (Transformation|GetWorldRotation _widgetlocation_2) (Math|Rotator|MakeRotator 0.0 9e+01 (Class|KismetMathLibrary|DegAtan2 (.y _returnvalue_9) (.x _returnvalue_9))) (* (Utilities|Time|GetWorldDeltaSeconds) 6.0) true) false false))))

(fn ConstructionScript)

(fn GetHorizontalVelocity
  (params (Target :type Scene%20Component%20Object%20Reference))
  (bind _returnvalue (Transformation|GetComponentVelocity Target))
  (return (Math|Vector2D|MakeVector2D (.x _returnvalue) (.y _returnvalue))))

(fn HorizontalVector
  (params (Vector :type Vector))
  (return (Math|Vector2D|MakeVector2D (.x Vector) (.y Vector))))

(fn ApplyDrunkLevel
  (params (Level :type Float%20%28single-precision%29))
  (Variables|Default|SetDrunkLevel Level)
  (Variables|Default|SetUpDraft (Math|Curves|GetFloatValue (Variables|Curves|GetCorrectiveForceCurve) Level))
  (Class|PrimitiveComponent|SetMassScale (Variables|Default|GetSphere) "None" (Math|Curves|GetFloatValue (Variables|Curves|GetFrictionCurve) Level))
  (Variables|Default|SetConstant%20Up (Math|Curves|GetFloatValue (Variables|Curves|GetConstantUpCurve) Level))
  (Variables|Default|SetAngleOffsetRange (Math|Curves|GetFloatValue (Variables|Curves|GetAngleOffsetCurve) Level))
  (Variables|Default|SetMaxSpeed (Math|Curves|GetFloatValue (Variables|Curves|GetMaxSpeedCurve) Level))
  (Variables|Default|SetRightStickForce (Math|Curves|GetFloatValue (Variables|Curves|GetRightStickCurve) Level))
  (Default|SetDrunkLevels (CallFunction|PostProcessontroller) (Variables|Default|GetDrunkLevel))
  (Default|SetIntensity (CallFunction|AudioController) (Variables|Default|GetDrunkLevel)))

(fn PostProcessontroller
  (bind _mandagamemode (Utilities|MandaGameMode)
    (:then
      (return (Variables|/Game/Manda/Framework/BP_MandaGameMode.BP_MandaGameMode_C|GetPostProcessController _mandagamemode)))))

(fn AudioController
  (bind _mandagamemode (Utilities|MandaGameMode)
    (:then
      (return (Variables|/Game/Manda/Framework/BP_MandaGameMode.BP_MandaGameMode_C|GetMusic_Crontroller _mandagamemode)))))