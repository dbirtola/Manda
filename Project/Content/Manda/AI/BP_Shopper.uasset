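; BP_Shopper is an AI-controlled shopper that picks up BP_Alcohol actors overlapping its pickup collider, attaching and tracking them.
; DashTowards faces a location and enables capsule physics for a timeline-scaled force dash; Tick disables physics once slow and no longer dashing.
; MoveTo and MoveToLocation issue AI moves with debug lines, the former only when not dashing, the latter only while dashing.
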(event OnComponentBeginOverlap(PickupCollider)
  (params (OverlappedComponent :type Primitive%20Component%20Object%20Reference) (OtherActor :type Actor%20Object%20Reference) (OtherComp :type Primitive%20Component%20Object%20Reference) (OtherBodyIndex :type Integer) (bFromSweep :type Boolean) (SweepResult :type Hit%20Result%20Structure%20%28by%20ref%29))
  (bind _asbp_alcohol (Utilities|Casting|CastToBP_Alcohol OtherActor))
  (Transformation|AttachActorToActor _asbp_alcohol self "None" "KeepWorld" "KeepRelative" "KeepRelative" true)
  (Utilities|Array|AddUnique (Variables|Default|GetAttachedAlcohol) _asbp_alcohol))

(event EventBeginPlay)

(event Collision|EventActorBeginOverlap
  (params (OtherActor :type Actor%20Object%20Reference)))

(event EventTick
  (params (DeltaSeconds :type Float%20%28single-precision%29))
  (if (and (not (Variables|Default|GetbDashing)) (< (Math|Vector|VectorLength (Transformation|GetVelocity)) 5e+01))
    (Physics|SetSimulatePhysics (Variables|Collision|GetCapsuleComponent) false)))

(fn ConstructionScript)

(fn DashTowards
  (params (Location :type Vector))
  (Variables|Default|SetDashDirection (Math|Vector|Normalize (- Location (Transformation|GetActorLocation))))
  (Transformation|SetActorRotation (Math|Rotator|FindLookatRotation (Transformation|GetActorLocation) Location))
  (Variables|Default|SetbDashing true)
  (Components|Timeline|PlayfromStart (Variables|Default|GetDashTimeline))
  (Physics|SetSimulatePhysics (Variables|Collision|GetCapsuleComponent) true))

(fn Moveto
  (params (Target :type Actor%20Object%20Reference))
  (if (not (Variables|Default|GetbDashing))
    (AI|Navigation|MovetoActor (AI|GetAIController self) Target -1.0 true true false 0)
    (Rendering|Debug|DrawDebugLine (Transformation|GetActorLocation) (Transformation|GetActorLocation Target) "(R=1.000000,G=0.000000,B=0.000000,A=1.000000)" 0.2 0.5)))

(fn MovetoLocation
  (params (Location :type Vector))
  (if (Variables|Default|GetbDashing)
    (AI|Navigation|MovetoLocation (AI|GetAIController self) Location -1.0 true true false false 0)
    (Rendering|Debug|DrawDebugLine (Transformation|GetActorLocation) Location "(R=1.000000,G=0.000000,B=0.000000,A=1.000000)" 0.2 0.5)))